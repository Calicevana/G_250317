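; BP_Char_3 is a player character with Enhanced Input look, jump and camera-relative movement that dies on hitting an actor tagged "Floor".
; BeginPlay adds the IMC_N_Context mapping, and the input actions drive controller rotation and character movement.
; A tagged capsule hit calls Die, which ragdolls the mesh, disables input and capsule collision.
; The spring arm then attaches to the mesh without collision testing, and the actor is destroyed after a short delay.
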(event OnComponentHit(CapsuleComponent)
  (params (HitComponent :type Primitive%20Component%20Object%20Reference) (OtherActor :type Actor%20Object%20Reference) (OtherComp :type Primitive%20Component%20Object%20Reference) (NormalImpulse :type Vector :default "0, 0, 0") (Hit :type Hit%20Result%20Structure%20%28by%20ref%29))
  (bind _springarm (Variables|Default|GetSpringArm))
  (if (Actor|ActorHasTag OtherActor "Floor")
    (CallFunction|Die)
    (Transformation|AttachComponentToComponent _springarm (Variables|Character|GetMesh) "None" "KeepRelative" "KeepRelative" "KeepRelative" true)
    (Variables|/Script/Engine.SpringArmComponent|SetbDoCollisionTest _springarm false)
    (Utilities|FlowControl|Delay 3.0)
    (Actor|DestroyActor)))

(event Custom|Die
  (bind _mesh (Variables|Character|GetMesh))
  (Physics|SetSimulatePhysics _mesh true)
  ;[1 1 1] 열거형 - 숫자를 나열 - 숫자에 이름을 붙인 것
  (Collision|SetCollisionEnabled _mesh "PhysicsOnly") ; 목록에 해당된 모드로 진입
  (Input|DisableInput (Game|GetPlayerController 0)) ; 1번을 눌러 모드로 진입하면 더이상 입력 받지 않게
  (Collision|SetCollisionEnabled (Variables|Collision|GetCapsuleComponent) "NoCollision"))

(event Input|EnhancedActionEvents|EnhancedInputActionIA_N_Jump
  (params (ActionValue :type Boolean) (ElapsedSeconds :type Float%20%28double-precision%29) (TriggeredSeconds :type Float%20%28double-precision%29) (InputAction :type Input%20Action%20Object%20Reference :default "/Game/BluePrint/Char_3/Input/IA_N_Jump.IA_N_Jump"))
  (:Started
    (Character|Jump))
  (:Completed
    (Character|StopJumping)))

(event Input|EnhancedActionEvents|EnhancedInputActionIA_N_Move
  (params (ActionValue :type Vector%202D%20Structure) (ElapsedSeconds :type Float%20%28double-precision%29) (TriggeredSeconds :type Float%20%28double-precision%29) (InputAction :type Input%20Action%20Object%20Reference :default "/Game/BluePrint/Char_3/Input/IA_N_Move.IA_N_Move"))
  (bind _returnvalue (Pawn|GetControlRotation :!class /Script/Engine.Pawn))
  (Pawn|Input|AddMovementInput (Math|Vector|GetRightVector (Math|Rotator|MakeRotator (.roll _returnvalue) 0.0 (.yaw _returnvalue))) (.x ActionValue) false)
  (Pawn|Input|AddMovementInput (Math|Vector|GetForwardVector (Math|Rotator|MakeRotator 0.0 0.0 (.yaw _returnvalue))) (.y ActionValue) false))

(event Input|EnhancedActionEvents|EnhancedInputActionIA_N_Look
  (params (ActionValue :type Vector%202D%20Structure) (ElapsedSeconds :type Float%20%28double-precision%29) (TriggeredSeconds :type Float%20%28double-precision%29) (InputAction :type Input%20Action%20Object%20Reference :default "/Game/BluePrint/Char_3/Input/IA_N_Look.IA_N_Look"))
  (Pawn|Input|AddControllerYawInput (.x ActionValue)) ; X - Yaw
  (Pawn|Input|AddControllerPitchInput (.y ActionValue)) ; Y축 - Pitch
)

(event EventBeginPlay
  (bind _asplayer_controller (Utilities|Casting|CastToPlayerController (Pawn|GetController)))
  (Utilities|IsValid (PlayerController|LocalPlayerSubsystems|GetEnhancedInputLocalPlayerSubsystem _asplayer_controller)
    (:Is%20Valid
      (Input|AddMappingContext (PlayerController|LocalPlayerSubsystems|GetEnhancedInputLocalPlayerSubsystem _asplayer_controller) "/Game/BluePrint/Char_3/Input/IMC_N_Context.IMC_N_Context" 0 "(bIgnoreAllPressedKeysUntilRelease=True,bForceImmediately=False,bNotifyUserSettings=False)"))))

(event Collision|EventActorBeginOverlap
  (params (OtherActor :type Actor%20Object%20Reference)))

(event EventTick
  (params (DeltaSeconds :type Float%20%28single-precision%29)))

(fn ConstructionScript)